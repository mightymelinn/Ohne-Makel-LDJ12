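; Base Blueprint for active abilities that target allies in the turn-based grid combat.
; Enabling or disabling the ability notifies the battle grid to toggle ally targeting, while the target slot is set directly or picked randomly from ally slots for AI.
; It gathers unique allies within Range of the target slot.
; Availability requires the parent check plus at least one ally slot on the grid, without testing range.
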(event `self.OnActiveAbilityEnabled`
  ;[1 1 1] Enable / disable ally slots
  (`/Game/TurnBasedStrategyRPGTemplate/Blueprints/Grid/BP_Grid.OnAllyTargetAbilityEnabled` (`/Game/TurnBasedStrategyRPGTemplate/Blueprints/Core/BP_BattleController.grid` (`self.battleController`))))

(event `self.OnActiveAbilityDisabled`
  ;[1 1 1] Enable / disable ally slots
  (`/Game/TurnBasedStrategyRPGTemplate/Blueprints/Grid/BP_Grid.OnAllyTargetAbilityDisabled` (`/Game/TurnBasedStrategyRPGTemplate/Blueprints/Core/BP_BattleController.grid` (`self.battleController`))))

(event `self.ResetTargetSlot`
  ;[1 1 1] Reset target slot
  (`self.SetTargetSlot` null))

(event `self.SetTargetSlot`
  (params (slot :type "/Game/TurnBasedStrategyRPGTemplate/Blueprints/Grid/Slots/BP_SlotBase Object Reference"))
  ;[1 1 1] Set target slot for the ability
  (set `self.targetSlot` slot))

(event `self.SetTargetSlotForAI`
  ;[1 1 1] Set target slot for the ability
  (set `self.targetSlot` (`KismetArrayLibrary.Array_Random` (`/Game/TurnBasedStrategyRPGTemplate/Blueprints/Grid/BP_Grid.allySlots` (`/Game/TurnBasedStrategyRPGTemplate/Blueprints/Core/BP_BattleController.grid` (`self.battleController`))))))

(fn `GetAbilitySlots`
  (returns (slotsInRange :type "Array of /Game/TurnBasedStrategyRPGTemplate/Blueprints/Grid/Slots/BP_SlotBase Object Reference") (emptySlotsInRange :type "Array of /Game/TurnBasedStrategyRPGTemplate/Blueprints/Grid/Slots/BP_SlotBase Object Reference") (alliesInRange :type "Array of /Game/TurnBasedStrategyRPGTemplate/Blueprints/Units/Characters/BP_CharacterBase Object Reference") (enemiesInRange :type "Array of /Game/TurnBasedStrategyRPGTemplate/Blueprints/Units/Characters/BP_CharacterBase Object Reference"))
  (locals (currentAllies :type "Array of /Game/TurnBasedStrategyRPGTemplate/Blueprints/Units/Characters/BP_CharacterBase Object Reference"))
  ;[1 1 1] Return allies
  (`/Engine/EditorBlueprintResources/StandardMacros.IsValid` (`self.targetSlot`)
    (:`Is Valid`
      (bind _slotsinrange (`/Game/TurnBasedStrategyRPGTemplate/Blueprints/Grid/BP_Grid.GetSlotsInRange` (`/Game/TurnBasedStrategyRPGTemplate/Blueprints/Core/BP_BattleController.grid` (`self.battleController`)) (`self.targetSlot`) (`self.range`) false))
      (for _array_element _slotsinrange
        (bind (_isallyslot _allycharacter) (`/Game/TurnBasedStrategyRPGTemplate/Blueprints/Grid/Slots/BP_SlotBase.IsAllySlot` _array_element (`self.abilityOwner`)))
        (if _isallyslot
          (`KismetArrayLibrary.Array_AddUnique` (`local.currentAllies`) _allycharacter))))
    (:`Is Not Valid`
      _))
  (return _ _ (`local.currentAllies`)))

(fn `IsAvailable`
  (params (isMeleeAttack :type Boolean))
  (returns (isAvailable :type Boolean))
  ;[1 1 1] Checks if there is an ally in range
  (bind _isavailable (`parent.IsAvailable` isMeleeAttack))
  (return (and _isavailable (> (`KismetArrayLibrary.Array_Length` (`/Game/TurnBasedStrategyRPGTemplate/Blueprints/Grid/BP_Grid.allySlots` (`/Game/TurnBasedStrategyRPGTemplate/Blueprints/Core/BP_BattleController.grid` (`self.battleController`)))) 0))))

(fn `UserConstructionScript`
  (`parent.UserConstructionScript`))