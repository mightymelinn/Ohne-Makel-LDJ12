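; Base aura ability for turn-based battles that buffs allies and debuffs enemies within range of its owner.
; ApplyAura queries the battle grid around the owner's slot, excluding the owner, and registers the aura on each slot in range.
; Each configured effect class is spawned as an actor for living targets, then added and initialized only if the target lacks it; duplicate actors are not destroyed here.
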(event `ApplyAura`
  ;[1 1 1] Add the aura to the slots in range and give buffs / debuffs to affected characters
  (bind (_slotsinrange _emptyslotsinrange _alliesinrange _enemiesinrange) (`/Game/TurnBasedStrategyRPGTemplate/Blueprints/Grid/BP_Grid.GetSlotsInCharacterRange` (`/Game/TurnBasedStrategyRPGTemplate/Blueprints/Core/BP_BattleController.grid` (`self.battleController`)) (`self.abilityOwner`) (`self.range`) (`/Game/TurnBasedStrategyRPGTemplate/Blueprints/Units/BP_UnitBase.slot` (`self.abilityOwner`)) true))
  (for _array_element _slotsinrange
    (`/Game/TurnBasedStrategyRPGTemplate/Blueprints/Grid/Slots/BP_SlotBase.AddAura` _array_element self (`self.abilityOwner`)))
  (for _array_element_2 _alliesinrange
    (`self.AddBuffsToCharacter` _array_element_2))
  (for _array_element_3 _enemiesinrange
    (`self.AddDebuffsToCharacter` _array_element_3)))

(event `AddBuffsToCharacter`
  (params (affectedCharacter :type "/Game/TurnBasedStrategyRPGTemplate/Blueprints/Units/Characters/BP_CharacterBase Object Reference"))
  ;[1 1 1] Add buffs to a character
  (for _array_element (`self.buffs`)
    (bind _isdead (`/Game/TurnBasedStrategyRPGTemplate/Blueprints/Units/Characters/BP_CharacterBase.IsDead` affectedCharacter))
    (if (not _isdead)
      (`self.AddBuff` affectedCharacter _array_element))))

(event `AddDebuffsToCharacter`
  (params (affectedCharacter :type "/Game/TurnBasedStrategyRPGTemplate/Blueprints/Units/Characters/BP_CharacterBase Object Reference"))
  ;[1 1 1] Add debuffs to a character
  (for _array_element (`self.debuffs`)
    (bind _isdead (`/Game/TurnBasedStrategyRPGTemplate/Blueprints/Units/Characters/BP_CharacterBase.IsDead` affectedCharacter))
    (if (not _isdead)
      (`self.AddDebuff` affectedCharacter _array_element))))

(event `AddBuff`
  (params (affectedCharacter :type "/Game/TurnBasedStrategyRPGTemplate/Blueprints/Units/Characters/BP_CharacterBase Object Reference") (buff :type "/Game/TurnBasedStrategyRPGTemplate/Blueprints/StatusEffects/Buffs/BP_BuffBase Class Reference"))
  ;[1 1 1] Add buff / debuff from the aura
  (bind _returnvalue (`|SpawnActorFromClass` buff (`KismetMathLibrary.MakeTransform` (0.0 0.0 0.0)) "Undefined" "SelectDefaultAtRuntime" null affectedCharacter 0 false true (`self.abilityOwner`) null))
  (bind _alreadygotbuff (`/Game/TurnBasedStrategyRPGTemplate/Blueprints/Units/Characters/BP_CharacterBase.AlreadyGotBuff` affectedCharacter _returnvalue))
  (if (not _alreadygotbuff)
    (`/Game/TurnBasedStrategyRPGTemplate/Blueprints/Units/Characters/BP_CharacterBase.AddBuff` affectedCharacter _returnvalue)
    (`/Game/TurnBasedStrategyRPGTemplate/Blueprints/StatusEffects/BP_StatusEffectBase.Initialize` _returnvalue)))

(event `AddDebuff`
  (params (affectedCharacter :type "/Game/TurnBasedStrategyRPGTemplate/Blueprints/Units/Characters/BP_CharacterBase Object Reference") (debuff :type "/Game/TurnBasedStrategyRPGTemplate/Blueprints/StatusEffects/Debuffs/BP_DebuffBase Class Reference"))
  ;[1 1 1] Add buff / debuff from the aura
  (bind _returnvalue (`|SpawnActorFromClass` debuff (`KismetMathLibrary.MakeTransform` (0.0 0.0 0.0)) "Undefined" "SelectDefaultAtRuntime" null affectedCharacter 0 false true (`self.abilityOwner`) null))
  (bind _alreadygotdebuff (`/Game/TurnBasedStrategyRPGTemplate/Blueprints/Units/Characters/BP_CharacterBase.AlreadyGotDebuff` affectedCharacter _returnvalue))
  (if (not _alreadygotdebuff)
    (`/Game/TurnBasedStrategyRPGTemplate/Blueprints/Units/Characters/BP_CharacterBase.AddDebuff` affectedCharacter _returnvalue)
    (`/Game/TurnBasedStrategyRPGTemplate/Blueprints/StatusEffects/BP_StatusEffectBase.Initialize` _returnvalue)))

(fn `UserConstructionScript`
  (`parent.UserConstructionScript`))