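; Base Blueprint for area-target spells in a turn-based strategy game, which affect grid slots around a chosen target slot.
; Enabling or disabling the spell notifies the battle controller's grid, and SetTargetSlot stores the center slot.
; GetSpellSlots queries the grid for slots within Range of that target and sorts them into empty slots, enemies and allies relative to the currently playing character.
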(event `self.OnSpellEnabled`
  ;[1 1 1] Enable / disable area target spell
  (`/Game/TurnBasedStrategyRPGTemplate/Blueprints/Grid/BP_Grid.OnAreaTargetSpellEnabled` (`/Game/TurnBasedStrategyRPGTemplate/Blueprints/Core/BP_BattleController.grid` (`self.battleController`)) self))

(event `self.OnSpellDisabled`
  ;[1 1 1] Enable / disable area target spell
  (`/Game/TurnBasedStrategyRPGTemplate/Blueprints/Grid/BP_Grid.OnAreaTargetSpellDisabled` (`/Game/TurnBasedStrategyRPGTemplate/Blueprints/Core/BP_BattleController.grid` (`self.battleController`))))

(event `self.SetTargetSlot`
  (params (slot :type "/Game/TurnBasedStrategyRPGTemplate/Blueprints/Grid/Slots/BP_SlotBase Object Reference"))
  ;[1 1 1] Set target slot for the spell
  (set `self.targetSlot` slot))

(fn `GetSpellSlots`
  (returns (slotsInRange :type "Array of /Game/TurnBasedStrategyRPGTemplate/Blueprints/Grid/Slots/BP_SlotBase Object Reference") (emptySlots :type "Array of /Game/TurnBasedStrategyRPGTemplate/Blueprints/Grid/Slots/BP_SlotBase Object Reference") (allies :type "Array of /Game/TurnBasedStrategyRPGTemplate/Blueprints/Units/Characters/BP_CharacterBase Object Reference") (enemies :type "Array of /Game/TurnBasedStrategyRPGTemplate/Blueprints/Units/Characters/BP_CharacterBase Object Reference"))
  (locals (currentEnemies :type "Array of /Game/TurnBasedStrategyRPGTemplate/Blueprints/Units/Characters/BP_CharacterBase Object Reference") (currentAllies :type "Array of /Game/TurnBasedStrategyRPGTemplate/Blueprints/Units/Characters/BP_CharacterBase Object Reference") (currentSlots :type "Array of /Game/TurnBasedStrategyRPGTemplate/Blueprints/Grid/Slots/BP_SlotBase Object Reference"))
  (bind _playingcharacter (`/Game/TurnBasedStrategyRPGTemplate/Blueprints/Core/BP_BattleController.playingCharacter` (`self.battleController`)))
  ;[1 1 1] Return all slots, empty slots, enemies and allies in range
  (`/Engine/EditorBlueprintResources/StandardMacros.IsValid` (`self.targetSlot`)
    (:`Is Valid`
      (bind _slotsinrange (`/Game/TurnBasedStrategyRPGTemplate/Blueprints/Grid/BP_Grid.GetSlotsInRange` (`/Game/TurnBasedStrategyRPGTemplate/Blueprints/Core/BP_BattleController.grid` (`self.battleController`)) (`self.targetSlot`) (`self.range`) false))
      (for _array_element _slotsinrange
        (if (`/Game/TurnBasedStrategyRPGTemplate/Blueprints/Grid/Slots/BP_SlotBase.IsEmpty` _array_element)
          (`KismetArrayLibrary.Array_AddUnique` (`local.currentSlots`) _array_element)
          (else
            (bind (_isenemyslot _enemycharacter) (`/Game/TurnBasedStrategyRPGTemplate/Blueprints/Grid/Slots/BP_SlotBase.IsEnemySlot` _array_element _playingcharacter))
            (if _isenemyslot
              (`KismetArrayLibrary.Array_AddUnique` (`local.currentEnemies`) _enemycharacter)
              (else
                (bind (_isallyslot _allycharacter) (`/Game/TurnBasedStrategyRPGTemplate/Blueprints/Grid/Slots/BP_SlotBase.IsAllySlot` _array_element _playingcharacter))
                (if _isallyslot
                  (`KismetArrayLibrary.Array_AddUnique` (`local.currentAllies`) _allycharacter))))))))
    (:`Is Not Valid`
      _))
  (return _slotsinrange (`local.currentSlots`) (`local.currentAllies`) (`local.currentEnemies`)))

(fn `UserConstructionScript`
  (`parent.UserConstructionScript`))