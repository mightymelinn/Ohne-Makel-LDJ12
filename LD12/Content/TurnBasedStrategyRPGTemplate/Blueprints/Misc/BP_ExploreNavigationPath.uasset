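; Actor that displays a navigation path between a start and target location, named for explore mode.
; ShowPath runs a synchronous navmesh query and rebuilds a spline through the path points, halving tangents to tighten curves.
; It then places instanced meshes at fixed intervals along the spline, rotating each toward the next and aligning the last with the spline.
; ClearPath destroys the actor.
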(event `ShowPath`
  (params (PathStart :type "Vector Structure (by ref)") (targetLocation :type "Vector Structure (by ref)"))
  (bind _pathspline (`self.PathSpline`))
  (bind _pathmesh (`self.PathMesh`))
  (bind _returnvalue (- (`InstancedStaticMeshComponent.GetInstanceCount` (`self.PathMesh`)) 1))
  (bind _outinstancetransform (`InstancedStaticMeshComponent.GetInstanceTransform` _pathmesh _returnvalue true))
  ;[1 1 1] Create navigation path
  (bind _returnvalue_2 (`NavigationSystemV1.FindPathToLocationSynchronously` PathStart targetLocation null null))
  (`SplineComponent.ClearSplinePoints` (`self.PathSpline`) true)
  (for (_array_element _array_index) (`NavigationPath.PathPoints` _returnvalue_2)
    (`SplineComponent.AddSplinePoint` _pathspline _array_element "World" true)
    (`SplineComponent.SetTangentsAtSplinePoint` (`self.PathSpline`) _array_index (* (`SplineComponent.GetArriveTangentAtSplinePoint` _pathspline _array_index "Local") 0.5) (* (`SplineComponent.GetLeaveTangentAtSplinePoint` _pathspline _array_index "Local") 0.5) "Local" true))
  (`InstancedStaticMeshComponent.ClearInstances` (`self.PathMesh`))
  (for _index (range (+ (`KismetMathLibrary.FFloor` (/ (`SplineComponent.GetSplineLength` (`self.PathSpline`)) 50.0)) 1))
    (bind _returnvalue_3 (`SplineComponent.GetLocationAtDistanceAlongSpline` (`self.PathSpline`) (* _index 50.0) "World"))
    (`InstancedStaticMeshComponent.AddInstanceWorldSpace` (`self.PathMesh`) (`KismetMathLibrary.MakeTransform` _returnvalue_3 (struct) (0.75 0.75 0.75)))
    (if (> _index 0)
      (bind _returnvalue_4 (- _index 1))
      (bind _outinstancetransform_2 (`InstancedStaticMeshComponent.GetInstanceTransform` (`self.PathMesh`) _returnvalue_4 true))
      (`InstancedStaticMeshComponent.UpdateInstanceTransform` (`self.PathMesh`) _returnvalue_4 (`KismetMathLibrary.MakeTransform` (.location _outinstancetransform_2) (`KismetMathLibrary.FindLookAtRotation` (.location _outinstancetransform_2) _returnvalue_3) (.scale _outinstancetransform_2)) true false false)))
  (`InstancedStaticMeshComponent.UpdateInstanceTransform` _pathmesh _returnvalue (`KismetMathLibrary.MakeTransform` (.location _outinstancetransform) (`SplineComponent.FindRotationClosestToWorldLocation` (`self.PathSpline`) (.location _outinstancetransform) "World") (.scale _outinstancetransform)) true false false))

(event `ClearPath`
  ;[1 1 1] Create navigation path
  (`self.K2_DestroyActor`))

(fn `UserConstructionScript`)