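; BP_Damage is a floating combat number actor that displays damage, healing or resurrection feedback through a widget component.
; On BeginPlay it passes its stack, damage, heal, element, AI and resurrect values to the WBP_DamageUI widget.
; It binds to the widget's OnShowed event and destroys itself once the display finishes.
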(event `self.ReceiveBeginPlay`
  (bind _aswbp_damage_ui (cast `/Game/TurnBasedStrategyRPGTemplate/Blueprints/Widgets/WBP_DamageUI` (`WidgetComponent.GetUserWidgetObject` (`self.DamageUI`)) :!pure true))
  ;[1 1 1] Show damage UI
  (add `/Game/TurnBasedStrategyRPGTemplate/Blueprints/Widgets/WBP_DamageUI.OnShowed` _aswbp_damage_ui (delegate `OnDamageShowedHandler`))
  (`/Game/TurnBasedStrategyRPGTemplate/Blueprints/Widgets/WBP_DamageUI.ShowDamage` _aswbp_damage_ui (`self.stack`) (`self.damage`) (`self.heal`) (`self.element`) (`self.isAI`) (`self.isResurrect`)))

(event `OnDamageShowedHandler`
  ;[1 1 1] Show damage UI
  (`self.K2_DestroyActor`))

(fn `UserConstructionScript`)