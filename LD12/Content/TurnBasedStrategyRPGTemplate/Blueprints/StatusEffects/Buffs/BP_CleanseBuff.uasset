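; BP_CleanseBuff is a status effect buff in a turn-based strategy RPG that clears debuffs from the affected character.
; On Initialize it walks the character's current debuffs in reverse, allowing safe removal during the loop.
; It removes only debuffs not granted by auras, and skips all removal if the cleanse itself comes from an aura.
; The buff then removes itself immediately, acting as an instant effect.
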(event `self.Initialize`
  ;[1 1 1] Removes all debuffs
  (bind (_arrayindex _arrayelement) (`/Engine/EditorBlueprintResources/StandardMacros.ReverseForEachLoop` (`/Game/TurnBasedStrategyRPGTemplate/Blueprints/Units/Characters/BP_CharacterBase.currentDebuffs` (`self.affectedCharacter`)))
    (:`LoopBody`
      (if (and (not (`/Game/TurnBasedStrategyRPGTemplate/Blueprints/StatusEffects/BP_StatusEffectBase.isFromAura` _arrayelement)) (not (`self.isFromAura`)))
        (`self.RemoveStatusEffect` _arrayelement)))
    (:`Completed`
      (`self.RemoveStatusEffect`))))

(fn `UserConstructionScript`
  (`parent.UserConstructionScript`))