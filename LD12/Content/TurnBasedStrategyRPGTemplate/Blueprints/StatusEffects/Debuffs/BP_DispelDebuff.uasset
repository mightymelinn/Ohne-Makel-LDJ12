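; BP_DispelDebuff is a one-shot debuff status effect for the turn-based strategy RPG template that strips buffs and debuffs.
; On Initialize it walks all status effects in reverse, so removals are safe mid-loop, and removes each one not granted by an aura.
; If the dispel itself comes from an aura, it removes none of the listed effects.
; It then removes itself in either case.
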(event `self.Initialize`
  ;[1 1 1] Removes all buffs and debuffs
  (bind _allstatuseffects (`self.GetAllStatusEffects`))
  (bind (_arrayindex _arrayelement) (`/Engine/EditorBlueprintResources/StandardMacros.ReverseForEachLoop` _allstatuseffects)
    (:`LoopBody`
      (if (and (not (`/Game/TurnBasedStrategyRPGTemplate/Blueprints/StatusEffects/BP_StatusEffectBase.isFromAura` _arrayelement)) (not (`self.isFromAura`)))
        (`self.RemoveStatusEffect` _arrayelement)))
    (:`Completed`
      (`self.RemoveStatusEffect`))))

(fn `UserConstructionScript`
  (`parent.UserConstructionScript`))