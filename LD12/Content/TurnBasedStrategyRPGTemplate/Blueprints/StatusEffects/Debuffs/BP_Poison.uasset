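; Poison debuff status effect that damages the affected character each turn as a fraction of its max health.
; On each DOT tick it rounds that fraction up, applies elemental reductions, and deals the result as elemental damage.
; It then signals that the DOT was applied, passing the hit montage length plus a short buffer, or just the buffer without a montage.
; The same element is reported for UI display.
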(event `self.OnDOT`
  (bind _affectedcharacter (`self.affectedCharacter`))
  (bind _mainstats_maxhealth (break `/Game/TurnBasedStrategyRPGTemplate/Blueprints/Structs/S_CharacterStats` (`/Game/TurnBasedStrategyRPGTemplate/Blueprints/Units/Characters/BP_CharacterBase.mainStats` (`self.affectedCharacter`))))
  ;[1 1 1] Take 10% damage every turn
  (`/Game/TurnBasedStrategyRPGTemplate/Blueprints/Units/Characters/BP_CharacterBase.TakeDamage` _affectedcharacter (`self.GetDamageAfterElementReductions` (`KismetMathLibrary.FCeil` (* _mainstats_maxhealth (`self.DOTAmount`))) "NewEnumerator2") "NewEnumerator2")
  (bind _gethitmontage (`/Game/TurnBasedStrategyRPGTemplate/Blueprints/Units/Characters/BP_CharacterBase.getHitMontage` _affectedcharacter)
    (:`then`
      (`self.OnDOTApplied` (+ (`AnimSequenceBase.SequenceLength` _gethitmontage) 0.5)))
    (:`else`
      (`self.OnDOTApplied` 0.5))))

(fn `ShowElementOnUI`
  (returns (NewParam :type "/Game/TurnBasedStrategyRPGTemplate/Blueprints/Enums/E_Element Enum"))
  ;[1 1 1] Show element info on UI
  (return "NewEnumerator2"))

(fn `UserConstructionScript`
  (`parent.UserConstructionScript`))