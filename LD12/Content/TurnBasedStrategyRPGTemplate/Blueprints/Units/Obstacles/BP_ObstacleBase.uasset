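; Base grid obstacle that occupies slots as a unit and can snap onto the grid from its construction script.
; When snapping, it finds overlapping slots, matches inner or outer slots to unit size parity, then claims and hides those it fits on and attaches to the grid.
; Resetting frees its slots and restores their type based on player spawn eligibility.
; Removal destroys the obstacle and its invisible obstacles.
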(event `ResetSlots`
  (params (actor :type "Actor Object Reference"))
  ;[1 1 1] Reset slots
  (`/Engine/EditorBlueprintResources/StandardMacros.IsValid` (`self.slot`)
    (:`Is Valid`
      (bind _values (`BlueprintMapLibrary.Map_Values` (`/Game/TurnBasedStrategyRPGTemplate/Blueprints/Grid/BP_Grid.slots` (`/Game/TurnBasedStrategyRPGTemplate/Blueprints/Grid/Slots/BP_SlotBase.grid` (`self.slot`)))))
      (for _array_element _values
        (if (== self (`/Game/TurnBasedStrategyRPGTemplate/Blueprints/Grid/Slots/BP_SlotBase.containedUnit` _array_element))
          (`/Game/TurnBasedStrategyRPGTemplate/Blueprints/Grid/Slots/BP_SlotBase.SetUnit` _array_element null)
          (if (`/Game/TurnBasedStrategyRPGTemplate/Blueprints/Grid/Slots/BP_SlotBase.canPlayerCharacterSpawn` _array_element)
            (`/Game/TurnBasedStrategyRPGTemplate/Blueprints/Grid/Slots/BP_SlotBase.SetSlotType` _array_element "NewEnumerator2" 1)
            (else
              (`/Game/TurnBasedStrategyRPGTemplate/Blueprints/Grid/Slots/BP_SlotBase.SetSlotType` _array_element "NewEnumerator1" 1)))))
      (set `self.slot` null))))

(event `RemoveObstacle`
  ;[1 1 1] Remove obstacle
  (for _array_element (`self.invisibleObstacles`)
    (`self.K2_DestroyActor` _array_element))
  (`self.K2_DestroyActor`))

(fn `UserConstructionScript`
  (locals (currentSlot :type "/Game/TurnBasedStrategyRPGTemplate/Blueprints/Grid/Slots/BP_Slot Object Reference"))
  (bind _currentslot (`local.currentSlot`))
  (bind _currentslot_2 (`local.currentSlot`))
  (bind _isinnerslot (`/Game/TurnBasedStrategyRPGTemplate/Blueprints/Grid/Slots/BP_Slot.isInnerSlot` (`local.currentSlot`)))
  (bind _returnvalue (== (mod (`self.unitSize`) 2) 0))
  ;[1 1 1] Snap on slots and set the data
  (`parent.UserConstructionScript`)
  (add `self.OnDestroyed` (`|CreateDelegate` :!event `ResetSlots`))
  (`self.ResetSlots` null)
  (if (`self.snapToGrid`)
    (bind _outactors (`KismetSystemLibrary.ComponentOverlapActors` (`self.Box`) (`SceneComponent.K2_GetComponentToWorld` (`self.Box`)) (`|MakeArray` "ObjectTypeQuery2" :!type "EObjectTypeQuery Enum") "/Game/TurnBasedStrategyRPGTemplate/Blueprints/Grid/Slots/BP_Slot.BP_Slot_C"))
    (if (> (`KismetArrayLibrary.Array_Length` _outactors) 0)
      (for _array_element _outactors
        (bind _asbp_slot (cast `/Game/TurnBasedStrategyRPGTemplate/Blueprints/Grid/Slots/BP_Slot` _array_element))
        (set `local.currentSlot` _asbp_slot)
        (if (or (and _isinnerslot _returnvalue) (and (not _isinnerslot) (not _returnvalue)))
          (`/Engine/EditorBlueprintResources/StandardMacros.IsValid` (`self.slot`)
            (:`Is Valid`
              (`self.ResetSlots` null))
            (:`Is Not Valid`
              _))
          (bind (_allslotsunitwillstandon _canunitfit) (`/Game/TurnBasedStrategyRPGTemplate/Blueprints/Grid/BP_Grid.CanUnitFitTo` (`/Game/TurnBasedStrategyRPGTemplate/Blueprints/Grid/Slots/BP_SlotBase.grid` _currentslot) _currentslot self))
          (if _canunitfit
            (for _array_element_2 _allslotsunitwillstandon
              (`/Game/TurnBasedStrategyRPGTemplate/Blueprints/Grid/Slots/BP_SlotBase.HideSlot` _array_element_2)
              (`/Game/TurnBasedStrategyRPGTemplate/Blueprints/Grid/Slots/BP_SlotBase.SetUnit` _array_element_2 self))
            (`SceneComponent.K2_SetWorldLocation` (`self.StaticMesh`) (`self.K2_GetActorLocation` (`local.currentSlot`)) false true)
            (`self.SetUnitAnchorSlot` (`BlueprintMapLibrary.Map_Find` (`/Game/TurnBasedStrategyRPGTemplate/Blueprints/Grid/BP_Grid.slots` (`/Game/TurnBasedStrategyRPGTemplate/Blueprints/Grid/Slots/BP_SlotBase.grid` _currentslot_2)) (`/Game/TurnBasedStrategyRPGTemplate/Blueprints/Grid/Slots/BP_SlotBase.coordinates` _currentslot_2)))
            (bind _output_get (set `self.grid` (`/Game/TurnBasedStrategyRPGTemplate/Blueprints/Grid/Slots/BP_SlotBase.grid` (`local.currentSlot`))))
            (`self.K2_AttachToActor` _output_get "None" "KeepWorld" "KeepWorld" "KeepWorld"))))
      (else
        (`self.ResetSlots` null)))))