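; Hexagonal grid slot for a turn-based strategy game that reacts to mouse clicks and hovering.
; Static mesh cursor events broadcast clicks with the pressed button and cursor exits with the slot itself, while cursor entry calls MouseOverSlot.
; The construction script sets the world scale of the mesh and the Paper sprite from separate slot size variables.
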(event `self.StaticMesh.OnClicked`
  (params (TouchedComponent :type "PrimitiveComponent Object Reference") (ButtonPressed :type "Key Structure"))
  (`self.OnSlotClicked` self ButtonPressed))

(event `self.StaticMesh.OnBeginCursorOver`
  (params (TouchedComponent :type "PrimitiveComponent Object Reference"))
  (`self.MouseOverSlot`))

(event `self.StaticMesh.OnEndCursorOver`
  (params (TouchedComponent :type "PrimitiveComponent Object Reference"))
  (`self.OnMouseLeaveSlot` self))

(fn `UserConstructionScript`
  (`SceneComponent.SetWorldScale3D` (`self.StaticMesh`) (`self.slotSize`))
  (`SceneComponent.SetWorldScale3D` (`self.PaperSprite`) (`self.slotSpriteSize`)))