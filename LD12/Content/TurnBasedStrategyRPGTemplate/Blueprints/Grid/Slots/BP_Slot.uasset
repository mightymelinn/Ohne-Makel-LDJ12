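; BP_Slot is a grid slot actor that turns mouse interaction on its collision box into slot events.
; Click, hover and leave are rebroadcast through dispatchers that pass the slot itself, plus the button on click and an inner-slot flag on hover.
; ClearAllCallbacks unbinds every listener from those three dispatchers.
; The construction script sizes the box and scales the Paper2D sprite from the slot's size variables.
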(event `self.Box.OnClicked`
  (params (TouchedComponent :type "PrimitiveComponent Object Reference") (ButtonPressed :type "Key Structure"))
  ;[1 1 1] Mouse events
  (`self.OnSlotClicked` self ButtonPressed))

(event `self.Box.OnBeginCursorOver`
  (params (TouchedComponent :type "PrimitiveComponent Object Reference"))
  ;[1 1 1] Mouse events
  (`self.MouseOverSlot`))

(event `MouseOverSlot`
  ;[1 1 1] Mouse events
  (`self.OnMouseOverSlot` self (`self.isInnerSlot`)))

(event `self.Box.OnEndCursorOver`
  (params (TouchedComponent :type "PrimitiveComponent Object Reference"))
  ;[1 1 1] Mouse events
  (`self.OnMouseLeaveSlot` self))

(event `self.ClearAllCallbacks`
  ;[1 1 1] Mouse events
  (clear `self.OnMouseOverSlot`)
  (clear `self.OnMouseLeaveSlot`)
  (clear `self.OnSlotClicked`))

(fn `UserConstructionScript`
  (`parent.UserConstructionScript`)
  (`BoxComponent.SetBoxExtent` (`self.Box`) (`self.slotSize`) true)
  (`SceneComponent.SetWorldScale3D` (`self.PaperSprite`) (`self.slotSpriteSize`)))